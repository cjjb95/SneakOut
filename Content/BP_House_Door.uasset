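; House door actor that swings open on demand and shows a widget while something overlaps its proximity sphere.
; The sphere's begin and end overlap events toggle the widget's visibility, without filtering the overlapping actor.
; OpenDoor fires DoorEvent, which plays a timeline that yaws the static mesh up to -90 degrees as its track reaches one.
; There is no closing path, and a debug "Hello" prints on every timeline update.
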(event OnComponentBeginOverlap(Sphere)
  (params (OverlappedComponent :type Primitive%20Component%20Object%20Reference) (OtherActor :type Actor%20Object%20Reference) (OtherComp :type Primitive%20Component%20Object%20Reference) (OtherBodyIndex :type Integer) (bFromSweep :type Boolean) (SweepResult :type Hit%20Result%20Structure%20%28by%20ref%29))
  (Rendering|SetVisibility (Variables|Default|GetWidget) true false))

(event OnComponentEndOverlap(Sphere)
  (params (OverlappedComponent :type Primitive%20Component%20Object%20Reference) (OtherActor :type Actor%20Object%20Reference) (OtherComp :type Primitive%20Component%20Object%20Reference) (OtherBodyIndex :type Integer))
  (Rendering|SetVisibility (Variables|Default|GetWidget) false false))

(event Custom|DoorEvent
  (bind _doortrack (Timeline|DoorTimer Play)
    (:Update
      (Transformation|SetRelativeRotation (Variables|Default|GetStaticMesh) (Math|Rotator|MakeRotator 0.0 0.0 (* _doortrack -9e+01)) false false)
      (Development|PrintString "Hello"))))

(fn ConstructionScript)

(fn OpenDoor
  (CallFunction|DoorEvent))